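; Player character Blueprint, named Player_controller, that handles movement, camera look, jumping, sprinting, health and death.
; Input axes and actions drive capsule-relative movement, controller yaw and pitch, and walk speed swaps while Sprint is held.
; BeginPlay creates and initializes the PlayerUI widget with a self reference.
; AnyDamage clamps health and calls EHealthUpdated, then at zero plays a death animation and disables input.
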(event `self.ReceiveBeginPlay`
  (bind _returnvalue (`|CreateWidget` "/Game/Blueprints/PlayerUI.PlayerUI_C"))
  (`UserWidget.AddToViewport` _returnvalue 0)
  (`/Game/Blueprints/PlayerUI.Initialize` _returnvalue self))

(event `InputAxis|Move forward`
  (params (AxisValue :type "Float (single-precision)"))
  ; Movement
  (`self.AddMovementInput` (`SceneComponent.GetForwardVector` (`self.CapsuleComponent`)) AxisValue))

(event `InputAction|Jump`
  (params (Key :type "Key Structure"))
  ; Actions
  (:`Pressed`
    (`self.Jump`)))

(event `InputAxis|Turn`
  (params (AxisValue :type "Float (single-precision)"))
  ; Camera
  (`self.AddControllerYawInput` AxisValue))

(event `self.ReceiveAnyDamage`
  (params (Damage :type "Float (single-precision)") (DamageType :type "DamageType Object Reference") (InstigatedBy :type "Controller Object Reference") (DamageCauser :type "Actor Object Reference"))
  (if (not (`self.IsDead`))
    (bind _output_get (set `self.CurrentHealth` (`KismetMathLibrary.FClamp` (- (`self.CurrentHealth`) Damage) 0.0 100.0)))
    (`self.E_HealthUpdated` _output_get (`self.MaxHealth`))
    (if (== _output_get 0.0)
      (set `self.IsDead` true)
      (`SkeletalMeshComponent.PlayAnimation` (`self.Mesh`) "/Game/Characters/Mannequins/Anims/Death/MM_Death_Front_01.MM_Death_Front_01" false)
      (`self.DisableInput` (`GameplayStatics.GetPlayerController` 0)))))

(event `InputAction|Sprint`
  (params (Key :type "Key Structure"))
  (bind _charactermovement (`self.CharacterMovement`))
  ; Actions
  (:`Pressed`
    (set `CharacterMovementComponent.MaxWalkSpeed` (`self.Sprint Speed`) _charactermovement))
  (:`Released`
    (set `CharacterMovementComponent.MaxWalkSpeed` (`self.Walk Speed`) _charactermovement)))

(event `InputAxis|Move right`
  (params (AxisValue :type "Float (single-precision)"))
  ; Movement
  (`self.AddMovementInput` (`SceneComponent.GetRightVector` (`self.CapsuleComponent`)) AxisValue))

(event `InputAxis|Look up`
  (params (AxisValue :type "Float (single-precision)"))
  ; Camera
  (`self.AddControllerPitchInput` AxisValue))

(fn `UserConstructionScript`)