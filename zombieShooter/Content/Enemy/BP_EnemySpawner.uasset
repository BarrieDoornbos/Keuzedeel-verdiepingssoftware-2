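; Enemy spawner actor that populates the navigable area around itself with AI_Enemy actors when play begins.
; SpawnEnemies picks random reachable points within SpawnRadius and spawns with collision handling set to always spawn, counting each in SpawnAmount.
; It re-calls itself after a short delay, retrying when no point is found, until SpawnAmount reaches SpawnTarget.
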(event `self.ReceiveBeginPlay`
  (`self.SpawnEnemies`))

(event `SpawnEnemies`
  (bind (_randomlocation _returnvalue) (`NavigationSystemV1.K2_GetRandomReachablePointInRadius` (`self.K2_GetActorLocation`) (`self.SpawnRadius`) null null))
  ; Spawn enemies
  (if (>= (`self.SpawnAmount`) (`self.SpawnTarget`))
    _
    (elif _returnvalue
      (`|SpawnActorFromClass` "/Game/Enemy/AI_Enemy.AI_Enemy_C" (`KismetMathLibrary.Conv_VectorToTransform` _randomlocation) "AlwaysSpawn" "MultiplyWithRoot" null null)
      (bind _result (`/Engine/EditorBlueprintResources/StandardMacros.IncrementInt` (`self.SpawnAmount`))
        (:`  `
          (set `self.SpawnAmount` _result)
          (`KismetSystemLibrary.Delay` 0.1)
          (`self.SpawnEnemies`)))
      (else
        (`KismetSystemLibrary.Delay` 0.1)
        (`self.SpawnEnemies`)))))

(fn `UserConstructionScript`)